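; Debug actor for the WFC plugin that lays out a TileSet's 3D tile assets in the world to show their edge socket types.
; Its construction script spawns a child actor component per tile def, spacing assets along X by their dimensions, and records each entry.
; When DrawOnTick is set, Tick draws a box and label on each socketed side, colored by a random color derived from the socket type.
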(event EventTick
  (params (DeltaSeconds :type Float%20%28single-precision%29))
  (if (Variables|Default|GetDrawOnTick)
    (CallFunction|DrawDebugAllTiles 0.0)))

(fn ConstructionScript
  (bind _gridunitsize (Variables|Default|GetGridUnitSize))
  (Variables|Default|SetRefresh false)
  (LocalVariables|SetNextTileLocation "0, 0, 0")
  (LocalVariables|SetHalfGridUnitSize (* (Variables|Default|GetGridUnitSize) 0.5))
  (bind _tileset (Variables|Default|GetTileSet)
    (:then
      (for _array_element (Variables|/Script/WFC.WFCTileSet|GetTileAssets _tileset)
        (bind _aswfctile_asset_3d (Utilities|Casting|CastToWFCTileAsset3D _array_element))
        (Utilities|FlowControl|Sequence
          (:then_0
            (for (_array_element_2 _array_index) (Variables|/Script/WFC.WFCTileAsset3D|GetTileDefs _aswfctile_asset_3d)
              (bind _returnvalue (AddComponent|AddChildActorComponent false (Math|Transform|MakeTransform (+ (LocalVariables|GetNextTileLocation) (* (.Location (Utilities|Struct|BreakWFCTileDef3D _array_element_2)) (Variables|Default|GetGridUnitSize))) "0, 0, 0" "1,1,1")))
              (ChildActorComponent|SetChildActorClass _returnvalue (.ActorClass (Utilities|Struct|BreakWFCTileDef3D _array_element_2)))
              (Utilities|Array|Add (Variables|Default|GetDebugTileEntries) (Utilities|Struct|MakeFDebugTileActor_BP _aswfctile_asset_3d _array_index _returnvalue))))
          (:then_1
            (LocalVariables|SetNextTileLocation (+ (LocalVariables|GetNextTileLocation) (Math|Vector|MakeVector (+ (* (.x (Variables|/Script/WFC.WFCTileAsset3D|GetDimensions _aswfctile_asset_3d)) (.x _gridunitsize)) (.x _gridunitsize)) 0.0 0.0)))))))
    (:else)))

(fn GetDebugBoxforSide
  (params (Side :type Integer)))

(fn GetTileCenterLocation
  (params (TileLocation :type Vector))
  (return (+ TileLocation (* (Variables|Default|GetGridUnitSize) 0.5))))

(fn DrawDebugTileSide
  (params (Direction :type Integer) (Type :type Integer) (Center :type Vector) (Duration :type Float%20%28single-precision%29))
  (bind _returnvalue (Class|WFCGrid3D|GetDirectionVector Direction))
  (bind _returnvalue_2 (CallFunction|GetRandomColorforInt Type))
  (bind _gridunitsize (Variables|Default|GetGridUnitSize))
  (bind _sideboxscale (Variables|Default|GetSideBoxScale))
  (bind _returnvalue_3 (Math|Float|Lerp _sideboxscale 1.0 0.75))
  (bind _returnvalue_4 (Math|Conversions|ToVector(Float) _returnvalue))
  (bind _returnvalue_5 (* _gridunitsize 0.5 _returnvalue_3))
  (LocalVariables|SetSideCenter (+ Center (* _returnvalue_4 _returnvalue_5)))
  (Rendering|Debug|DrawDebugBox (LocalVariables|GetSideCenter) (* (CallFunction|OneMinusVector (Math|Vector|VectorGetAbs _returnvalue_4)) _returnvalue_5 _sideboxscale) _returnvalue_2 "0, 0, 0" Duration (Variables|Default|GetThickness))
  (Rendering|Debug|DrawDebugString (LocalVariables|GetSideCenter) (Utilities|String|ToString(Integer) Type) 0 _returnvalue_2 Duration))

(fn DrawDebugTileSides
  (params (TileAsset :type WFC%20Tile%20Asset%20Object%20Reference) (TileDefIndex :type Integer) (TileActorLocation :type Vector) (Duration :type Float%20%28single-precision%29))
  (bind _aswfctile_asset_3d (Utilities|Casting|CastToWFCTileAsset3D TileAsset))
  (bind _output_get (LocalVariables|SetTileDef3D (Class|WFCTileAsset3D|GetTileDefbyIndex _aswfctile_asset_3d TileDefIndex)))
  (bind _keys (Utilities|Map|Keys (.EdgeSocketTypes (Utilities|Struct|BreakWFCTileDef3D _output_get))))
  (for _array_element _keys
    (CallFunction|DrawDebugTileSide (Math|Conversions|ToInteger(Byte) _array_element) (.Value (Utilities|Map|Find (.EdgeSocketTypes (Utilities|Struct|BreakWFCTileDef3D _output_get)) _array_element)) (CallFunction|GetTileCenterLocation TileActorLocation) Duration)))

(fn DrawDebugAllTiles
  (params (Duration :type Float%20%28single-precision%29))
  (for _array_element (Variables|Default|GetDebugTileEntries)
    (CallFunction|DrawDebugTileSides (.TileAsset (Utilities|Struct|BreakFDebugTileActor_BP _array_element)) (.TileDefIndex (Utilities|Struct|BreakFDebugTileActor_BP _array_element)) (Transformation|GetWorldLocation (.TileActorComponent (Utilities|Struct|BreakFDebugTileActor_BP _array_element))) Duration)))