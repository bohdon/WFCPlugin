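; A Blueprint library of small static helpers in the WFC plugin's debug folder.
; GetRandomColorForInt maps an integer to a repeatable color by seeding a random stream with it and picking a hue at fixed saturation and value.
; The hue is drawn over a wider range and wrapped to 360 degrees to improve color spread.
; OneMinusVector returns one minus each component of a vector.
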(fn GetRandomColorforInt
  (params (Value :type Integer))
  (return (Class|KismetMathLibrary|HSVtoRGB (Math|Float|%(Float) (* (Math|Random|RandomFloatfromStream (Math|Random|MakeRandomStream Value)) 1.08e+03) 3.6e+02) 0.9 0.7 1.0)))

(fn OneMinusVector
  (params (Vector :type Vector))
  (bind (_x _y _z) (Math|Vector|BreakVector Vector))
  (return (Math|Vector|MakeVector (- 1.0 _x) (- 1.0 _y) (- 1.0 _z))))