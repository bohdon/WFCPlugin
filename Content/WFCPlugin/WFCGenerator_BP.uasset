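; Test harness actor for a 2D Wave Function Collapse generator that spawns actors for the selected tiles on a grid.
; RegenerateTileActors rebuilds every tile from the results, placed relative to the actor with grid scaling and 90-degree rotation steps.
; A cell-selected event spawns tiles incrementally as generation advances.
; On BeginPlay it either auto-runs or initializes; hotkeys step, run, reset, or toggle a looping timer that restarts finished or failed runs.
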(event OnCellSelectedEventBP(WFCGenerator)
  (params (CellIndex :type Integer))
  (bind _outtiles (Class|WFCGeneratorComponent|GetSelectedTiles (Variables|Default|GetWFCGenerator)))
  (bind _aswfctile_2d_asset (Utilities|Casting|CastToWFCTile2dAsset (.Object (Utilities|Struct|BreakWFCTile (Utilities|Array|Get(acopy) _outtiles CellIndex)))))
  (bind _returnvalue (Game|SpawnActorfromClass (Variables|/Script/WFC.WFCTile2dAsset|GetActorClass _aswfctile_2d_asset) (Math|Transform|ComposeTransforms (Math|Transform|MakeTransform (* (Math|Conversions|ToVector2D(IntPoint) (Class|WFCGrid2D|GetLocationforCellIndex (.AsWFCGrid%202D (Utilities|Casting|CastToWFCGrid2D (Class|WFCGeneratorComponent|GetGrid (Variables|Default|GetWFCGenerator)))) CellIndex)) (Variables|Default|GetGridUnitSize)) (Math|Rotator|MakeRotator 0.0 0.0 (* (.Rotation (Utilities|Struct|BreakWFCTile (Utilities|Array|Get(acopy) _outtiles CellIndex))) 9e+01))) (Transformation|GetActorTransform)) "Undefined" 0 0))
  (Utilities|Array|Add (Variables|Default|GetSpawnedActors) _returnvalue))

(event Custom|RegenerateTileActors
  (bind _wfcgenerator (Variables|Default|GetWFCGenerator))
  (CallFunction|DestroySpawnedActors)
  (bind _aswfcgrid_2d (Utilities|Casting|CastToWFCGrid2D (Class|WFCGeneratorComponent|GetGrid _wfcgenerator)))
  (bind _outtiles (Class|WFCGeneratorComponent|GetSelectedTiles _wfcgenerator))
  (for (_array_element _array_index) _outtiles
    (bind _aswfctile_2d_asset (Utilities|Casting|CastToWFCTile2dAsset (.Object (Utilities|Struct|BreakWFCTile _array_element))))
    (bind _returnvalue (Game|SpawnActorfromClass (Variables|/Script/WFC.WFCTile2dAsset|GetActorClass _aswfctile_2d_asset) (Math|Transform|ComposeTransforms (Math|Transform|MakeTransform (* (Math|Conversions|ToVector2D(IntPoint) (Class|WFCGrid2D|GetLocationforCellIndex _aswfcgrid_2d _array_index)) (Variables|Default|GetGridUnitSize)) (Math|Rotator|MakeRotator 0.0 0.0 (* (.Rotation (Utilities|Struct|BreakWFCTile _array_element)) 9e+01))) (Transformation|GetActorTransform)) "Undefined" 0 0))
    (Utilities|Array|Add (Variables|Default|GetSpawnedActors) _returnvalue)))

(event Custom|DestroySpawnedActors
  (for _array_element (Variables|Default|GetSpawnedActors)
    (Actor|DestroyActor _array_element))
  (Utilities|Array|Clear (Variables|Default|GetSpawnedActors)))

(event Custom|OnNextTimer
  (CallFunction|NextorRestart))

(event Custom|NextOrRestart
  (bind _wfcgenerator (Variables|Default|GetWFCGenerator))
  (bind _generator (Variables|/Script/WFC.WFCGeneratorComponent|GetGenerator _wfcgenerator))
  (switch Utilities|FlowControl|Switch|SwitchonEWFCGeneratorState (Class|WFCGeneratorComponent|GetState _wfcgenerator)
    (:None
      (Class|WFCGeneratorComponent|InitializeGenerator _wfcgenerator :!label _label)
      (CallFunction|DestroySpawnedActors)
      (Class|WFCGenerator|Next _generator))
    (:InProgress
      (Class|WFCGenerator|Next _generator))
    (:Finished
      (goto _label))
    (:Error
      (goto _label))))

(event EventBeginPlay
  (bind _wfcgenerator (Variables|Default|GetWFCGenerator))
  (Input|EnableInput (Game|GetPlayerController 0))
  (if (Variables|/Script/WFC.WFCGeneratorComponent|GetbAutoRun _wfcgenerator)
    (CallFunction|RegenerateTileActors)
    (else
      (Class|WFCGeneratorComponent|InitializeGenerator _wfcgenerator))))

(event Input|KeyboardEvents|SpaceBar
  (params (Key :type Key%20Structure :default "None"))
  (:Pressed
    (Utilities|FlowControl|FlipFlop
      (:A
        (bind _returnvalue (Utilities|Time|SetTimerbyEvent (delegate Custom|OnNextTimer) (Variables|Default|GetNextTimerInterval) true))
        (Variables|Default|SetNextTimer _returnvalue))
      (:B
        (Utilities|Time|ClearandInvalidateTimerbyHandle (Variables|Default|GetNextTimer))))))

(event Input|MouseEvents|MouseWheelUp
  (params (Key :type Key%20Structure :default "None"))
  (:Pressed
    (Class|WFCGenerator|Next (Variables|/Script/WFC.WFCGeneratorComponent|GetGenerator (Variables|Default|GetWFCGenerator)))))

(event Input|KeyboardEvents|Period
  (params (Key :type Key%20Structure :default "None"))
  (:Pressed
    (Class|WFCGeneratorComponent|Run (Variables|Default|GetWFCGenerator))
    (CallFunction|RegenerateTileActors)))

(event Input|KeyboardEvents|Backspace
  (params (Key :type Key%20Structure :default "None"))
  (:Pressed
    (Class|WFCGeneratorComponent|InitializeGenerator (Variables|Default|GetWFCGenerator))
    (CallFunction|DestroySpawnedActors)))

(fn ConstructionScript)