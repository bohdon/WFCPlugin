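; Actor that runs a Wave Function Collapse generator component and spawns the selected tiles as actors on a 2D or 3D grid.
; Each cell selection spawns its tile's actor class, yawed in quarter turns around a corner or center pivot; regeneration destroys and rebuilds all spawned actors.
; Keys step, fully run, reset or toggle timed auto-stepping that restarts when finished or failed.
; A Debug flag draws color-coded candidate counts per cell.
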(event OnCellSelectedEventBP(WFCGenerator)
  (params (CellIndex :type Integer))
  (bind _wfcgenerator (Variables|Default|GetWFCGenerator))
  (bind (_bsuccess _tileid) (Class|WFCGeneratorComponent|GetSelectedTileId _wfcgenerator CellIndex))
  (if _bsuccess
    (bind _aswfcasset_model (Utilities|Casting|CastToWFCAssetModel (Variables|/Script/WFC.WFCGeneratorComponent|GetModel _wfcgenerator)))
    (CallFunction|SpawnTileActor (Class|WFCTileModel2D|GetTilebyId _aswfcasset_model _tileid) CellIndex)))

(event Custom|RegenerateTileActors
  (bind _wfcgenerator (Variables|Default|GetWFCGenerator))
  (CallFunction|DestroySpawnedActors)
  (bind _tileids (Class|WFCGeneratorComponent|GetSelectedTileIds _wfcgenerator))
  (bind _aswfcasset_model (Utilities|Casting|CastToWFCAssetModel (Variables|/Script/WFC.WFCGeneratorComponent|GetModel _wfcgenerator)))
  (for (_array_element _array_index) _tileids
    (CallFunction|SpawnTileActor (Class|WFCTileModel2D|GetTilebyId _aswfcasset_model _array_element) _array_index)))

(event Custom|DestroySpawnedActors
  (for _array_element (Variables|Default|GetSpawnedActors)
    (Actor|DestroyActor _array_element))
  (Utilities|Array|Clear (Variables|Default|GetSpawnedActors)))

(event Custom|OnNextTimer
  (CallFunction|NextorRestart))

(event Custom|NextOrRestart
  (bind _wfcgenerator (Variables|Default|GetWFCGenerator))
  (bind _generator (Variables|/Script/WFC.WFCGeneratorComponent|GetGenerator _wfcgenerator))
  (switch Utilities|FlowControl|Switch|SwitchonEWFCGeneratorState (Class|WFCGeneratorComponent|GetState _wfcgenerator)
    (:None
      (Class|WFCGeneratorComponent|InitializeGenerator _wfcgenerator :!label _label)
      (CallFunction|DestroySpawnedActors)
      (Class|WFCGenerator|Next _generator))
    (:InProgress
      (Class|WFCGenerator|Next _generator))
    (:Finished
      (goto _label))
    (:Error
      (goto _label))))

(event EventTick
  (params (DeltaSeconds :type Float%20%28single-precision%29))
  (bind _wfcgenerator (Variables|Default|GetWFCGenerator))
  (bind _generator (Variables|/Script/WFC.WFCGeneratorComponent|GetGenerator _wfcgenerator))
  (if (Variables|Default|GetDebug)
    (Variables|Default|SetNumTiles (Class|WFCGenerator|GetNumTiles _generator))
    (bind _output_get (Variables|Default|SetNumCells (Class|WFCGenerator|GetNumCells _generator)))
    (for _index (range 0 (- _output_get 1))
      (bind _returnvalue (Class|WFCGenerator|GetNumCellCandidates _generator _index))
      (bind _returnvalue_2 (CallFunction|GetSelectedTileName _index))
      (Rendering|Debug|DrawDebugString (Math|Transform|TransformLocation (Transformation|GetActorTransform) (+ (* (CallFunction|GetLocationforCellIndex _index) (Variables|Default|GetGridUnitSize)) (Math|Vector|SelectVector "0, 0, 0" (* (Variables|Default|GetGridUnitSize) 0.5) (Variables|Default|GetTilesUseCenterPivot)))) (Utilities|String|ToString(Text) (Utilities|Text|FormatText "{cell} 
{tileinfo}" (Class|WFCGrid|GetCellName (Class|WFCGeneratorComponent|GetGrid _wfcgenerator) _index) (Utilities|String|SelectString _returnvalue_2 (Utilities|String|ToString(Integer) _returnvalue) (== _returnvalue 1)))) 0 (Math|Color|SelectColor "(R=0.000000,G=0.052807,B=1.000000,A=1.000000)" (Math|Color|SelectColor "(R=1.000000,G=0.000000,B=0.000000,A=1.000000)" (Math|Color|Lerp(LinearColor) "(R=0.000000,G=1.000000,B=0.108455,A=1.000000)" "(R=1.000000,G=0.604231,B=0.000000,A=1.000000)" (/ (Math|Conversions|ToFloat(Integer) _returnvalue) (Math|Conversions|ToFloat(Integer) (Variables|Default|GetNumTiles)))) (== _returnvalue 0)) (== _returnvalue 1))))))

(event EventBeginPlay
  (bind _wfcgenerator (Variables|Default|GetWFCGenerator))
  (Input|EnableInput (Game|GetPlayerController 0))
  (if (Variables|/Script/WFC.WFCGeneratorComponent|GetbAutoRun _wfcgenerator)
    (CallFunction|RegenerateTileActors)
    (else
      (Class|WFCGeneratorComponent|InitializeGenerator _wfcgenerator))))

(event Input|KeyboardEvents|SpaceBar
  (params (Key :type Key%20Structure :default "None"))
  (:Pressed
    (Utilities|FlowControl|FlipFlop
      (:A
        (bind _returnvalue (Utilities|Time|SetTimerbyEvent (delegate Custom|OnNextTimer) (Variables|Default|GetNextTimerInterval) true))
        (Variables|Default|SetNextTimer _returnvalue))
      (:B
        (Utilities|Time|ClearandInvalidateTimerbyHandle (Variables|Default|GetNextTimer))))))

(event Input|MouseEvents|MouseWheelUp
  (params (Key :type Key%20Structure :default "None"))
  (:Pressed
    (Class|WFCGenerator|Next (Variables|/Script/WFC.WFCGeneratorComponent|GetGenerator (Variables|Default|GetWFCGenerator)))))

(event Input|KeyboardEvents|Period
  (params (Key :type Key%20Structure :default "None"))
  (:Pressed
    (Class|WFCGeneratorComponent|Run (Variables|Default|GetWFCGenerator))
    (CallFunction|RegenerateTileActors)))

(event Input|KeyboardEvents|Backspace
  (params (Key :type Key%20Structure :default "None"))
  (:Pressed
    (Class|WFCGeneratorComponent|InitializeGenerator (Variables|Default|GetWFCGenerator))
    (CallFunction|DestroySpawnedActors)))

(fn ConstructionScript)

(fn GetLocationforCellIndex
  (params (CellIndex :type Integer))
  (bind _wfcgenerator (Variables|Default|GetWFCGenerator))
  (bind _returnvalue (Class|WFCGeneratorComponent|GetGrid _wfcgenerator))
  (bind _aswfcgrid_3d (Utilities|Casting|CastToWFCGrid3D _returnvalue)
    (:then
      (return (Class|WFCGrid3D|GetLocationforCellIndex _aswfcgrid_3d CellIndex)))
    (:CastFailed
      (bind _aswfcgrid_2d (Utilities|Casting|CastToWFCGrid2D _returnvalue)
        (:then
          (return (Utilities|Struct|MakeIntVector (.x (Class|WFCGrid2D|GetLocationforCellIndex _aswfcgrid_2d CellIndex)) (.y (Class|WFCGrid2D|GetLocationforCellIndex _aswfcgrid_2d CellIndex)) 0)))
        (:CastFailed
          (return ""))))))

(fn SpawnTileActor
  (params (ModelTile :type WFC%20Model%20Asset%20Tile%20Structure%20%28by%20ref%29) (CellIndex :type Integer))
  (bind (_rotation _tileasset _tiledefindex) (Utilities|Struct|BreakWFCModelAssetTile ModelTile))
  (bind _actorclass (CallFunction|GetTileAssetActorClass _tileasset _tiledefindex))
  (if (Utilities|IsValidClass _actorclass)
    (bind _returnvalue (Game|SpawnActorfromClass _actorclass (Math|Transform|ComposeTransforms (CallFunction|MakeTileRotationTransform (Math|Rotator|MakeRotator 0.0 0.0 (* _rotation 9e+01))) (Math|Transform|ComposeTransforms (Math|Transform|MakeTransform (* (CallFunction|GetLocationforCellIndex CellIndex) (Variables|Default|GetGridUnitSize))) (Transformation|GetActorTransform))) "Undefined" 0 0))
    (Utilities|Array|Add (Variables|Default|GetSpawnedActors) _returnvalue)))

(fn GetTileAssetActorClass
  (params (TileAsset :type WFC%20Tile%20Asset%20Object%20Reference) (TileDefIndex :type Integer))
  (bind _aswfctile_asset_3d (Utilities|Casting|CastToWFCTileAsset3D TileAsset)
    (:then
      (return (Utilities|Struct|BreakWFCTileDef3D (Class|WFCTileAsset3D|GetTileDefbyIndex _aswfctile_asset_3d TileDefIndex))))
    (:CastFailed
      (bind _aswfctile_asset_2d (Utilities|Casting|CastToWFCTileAsset2D TileAsset))
      (return (Utilities|Struct|BreakWFCTileDef2D (Class|WFCTileAsset2D|GetTileDefbyIndex _aswfctile_asset_2d TileDefIndex))))))

(fn MakeTileRotationTransform
  (params (Rotation :type Rotator))
  (bind _gridunitsize (Variables|Default|GetGridUnitSize))
  (bind _returnvalue (* _gridunitsize 0.5))
  (bind _returnvalue_2 (Math|Transform|MakeTransform _returnvalue))
  (if (Variables|Default|GetTilesUseCenterPivot)
    (return (Math|Transform|MakeTransform "0, 0, 0" Rotation))
    (else
      (return (Math|Transform|ComposeTransforms (Math|Transform|ComposeTransforms (Math|Transform|InvertTransform _returnvalue_2) (Math|Transform|MakeTransform "0, 0, 0" Rotation)) _returnvalue_2)))))

(fn GetSelectedTile
  (params (CellIndex :type Integer))
  (bind _wfcgenerator (Variables|Default|GetWFCGenerator))
  (bind _aswfcasset_model (Utilities|Casting|CastToWFCAssetModel (Variables|/Script/WFC.WFCGeneratorComponent|GetModel _wfcgenerator)))
  (bind (_bsuccess _tileid) (Class|WFCGeneratorComponent|GetSelectedTileId _wfcgenerator CellIndex))
  (if _bsuccess
    (return (Class|WFCAssetModel|GetTilebyId _aswfcasset_model _tileid))
    (else
      (return ""))))

(fn GetSelectedTileName
  (params (CellIndex :type Integer))
  (bind _returnvalue (CallFunction|GetSelectedTile CellIndex))
  (Utilities|IsValid (.TileAsset (Utilities|Struct|BreakWFCModelAssetTile _returnvalue))
    (:Is%20Valid
      (return (Utilities|String|ToString(Text) (Utilities|Text|FormatText "[{id}]" (.Id (Utilities|Struct|BreakWFCModelAssetTile _returnvalue))))))))